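; Player pawn with camera-relative movement, yaw turning, and a gun held as a child actor that starts and stops firing with the left mouse button.
; On BeginPlay it caches the gun, clamps camera pitch and registers its spawn transform with BP_GameMode.
; Health changes print the updated value, and on death it asks the game mode to respawn before destroying itself.
; LookUp is unwired, so pitch input has no effect.
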(event EventBeginPlay
  (bind _returnvalue (Game|GetPlayerCameraManager 0))
  (Utilities|FlowControl|Sequence
    (:then_0
      ;[1 1 1] Get Gun Actor
      (bind _asbp_gun (Utilities|Casting|CastToBP_Gun (Variables|/Script/Engine.ChildActorComponent|GetChildActor (Variables|Default|GetGunActor))))
      (Variables|Default|SetGun _asbp_gun)
      ;[1 1 1] Camera Clamp
      (Variables|/Script/Engine.PlayerCameraManager|SetViewPitchMax _returnvalue 4e+01)
      (Variables|/Script/Engine.PlayerCameraManager|SetViewPitchMin _returnvalue -4e+01))
    (:then_1
      ;[1 1 1] Spawn position
      (bind _asbp_game_mode (Utilities|Casting|CastToBP_GameMode (Game|GetGameMode)))
      (bind _output_get (Variables|Default|SetAs%20BP%20Game%20Mode _asbp_game_mode))
      (Default|SetPlayerSpawnTransform _output_get (Transformation|GetActorTransform)))))

(event EventAffectHealth
  (params (Delta :type Float%20%28single-precision%29))
  ;[1 1 1] Update Player Health
  (bind _newhealth (CallFunction|UpdateHealthPoints Delta))
  (Development|PrintString (Utilities|String|ToString(Float) _newhealth))
  (if (Variables|Default|GetbIsDead)
    (Default|RespawnPlayer (Variables|Default|GetAs%20BP%20Game%20Mode))
    (Actor|DestroyActor)))

(event Input|AxisEvents|InputAxisMoveForward
  (params (AxisValue :type Float%20%28single-precision%29))
  ;[1 1 1] Move Inputs
  (Pawn|Input|AddMovementInput (Math|Vector|GetForwardVector (Variables|Default|GetCamera)) AxisValue false))

(event Input|AxisEvents|InputAxisMoveRight
  (params (AxisValue :type Float%20%28single-precision%29))
  ;[1 1 1] Move Inputs
  (Pawn|Input|AddMovementInput (Math|Vector|GetRightVector (Variables|Default|GetCamera)) AxisValue false))

(event Input|AxisEvents|InputAxisLookUp
  (params (AxisValue :type Float%20%28single-precision%29))
  ;[1 1 1] Rotate Player
)

(event Input|AxisEvents|InputAxisTurn
  (params (AxisValue :type Float%20%28single-precision%29))
  ;[1 1 1] Rotate Player
  (Pawn|Input|AddControllerYawInput AxisValue))

(event Input|MouseEvents|LeftMouseButton
  (params (Key :type Key%20Structure :default "None"))
  (bind _gun (Variables|Default|GetGun))
  ;[1 1 1] Shoot
  (:Pressed
    (Default|StartFiring _gun))
  (:Released
    (Default|StopFiring _gun)))

(fn ConstructionScript
  (|CallParentFunction))