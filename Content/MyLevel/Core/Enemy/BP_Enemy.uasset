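; BP_Enemy is an enemy actor that damages the player on overlap and can itself be killed.
; When BP_Player enters HitTarget, a looping timer deals DamageAmount at a rate set by AttackPerSec, and is cleared when that player leaves.
; Incoming AffectHealth calls go through UpdateHealthPoints, print the result, and destroy the actor once IsDead is true.
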(event OnComponentBeginOverlap(HitTarget)
  (params (OverlappedComponent :type Primitive%20Component%20Object%20Reference) (OtherActor :type Actor%20Object%20Reference) (OtherComp :type Primitive%20Component%20Object%20Reference) (OtherBodyIndex :type Integer) (bFromSweep :type Boolean) (SweepResult :type Hit%20Result%20Structure%20%28by%20ref%29))
  ;[1 1 1] Attack Player
  (bind _asbp_player (Utilities|Casting|CastToBP_Player OtherActor))
  (Variables|Default|SetPlayer _asbp_player)
  (bind _returnvalue (Utilities|Time|SetTimerbyEvent (delegate Custom|DamageHero) (/ 1.0 (Variables|Default|GetAttackPerSec)) true))
  (Variables|Default|SetTimer _returnvalue))

(event OnComponentEndOverlap(HitTarget)
  (params (OverlappedComponent :type Primitive%20Component%20Object%20Reference) (OtherActor :type Actor%20Object%20Reference) (OtherComp :type Primitive%20Component%20Object%20Reference) (OtherBodyIndex :type Integer))
  ;[1 1 1] Stop Attack
  (if (== OtherActor (Variables|Default|GetPlayer))
    (Utilities|Time|ClearandInvalidateTimerbyHandle (Variables|Default|GetTimer))))

(event Custom|DamageHero
  ;[1 1 1] Attack Player
  (Default|AffectHealth (Variables|Default|GetPlayer) (Variables|Default|GetDamageAmount)))

(event EventBeginPlay
  (|CallParentFunction) ; This node is disabled and will not be called.\nDrag off pins to build functionality.
)

(event Collision|EventActorBeginOverlap
  (params (OtherActor :type Actor%20Object%20Reference))
  (|CallParentFunction OtherActor) ; This node is disabled and will not be called.\nDrag off pins to build functionality.
)

(event EventTick
  (params (DeltaSeconds :type Float%20%28single-precision%29))
  (|CallParentFunction DeltaSeconds) ; This node is disabled and will not be called.\nDrag off pins to build functionality.
)

(event EventAffectHealth
  (params (Delta :type Float%20%28single-precision%29))
  ;[1 1 1] Take Damage
  (bind _newhealth (CallFunction|UpdateHealthPoints Delta))
  (Development|PrintString (Utilities|String|ToString(Float) _newhealth))
  (if (Variables|Default|GetbIsDead)
    (Actor|DestroyActor)))

(fn ConstructionScript
  (|CallParentFunction))