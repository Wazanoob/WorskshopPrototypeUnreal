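; BP_Character is a character Blueprint that tracks health points and whether the character is dead.
; UpdateHealthPoints adds a signed delta to HealthPoints without clamping, sets IsDead when the total is zero or below, and returns the new value.
; A separate UpdateIsDead event repeats the same death check on the current health without changing it.
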(event Custom|UpdateIsDead
  ;[1 1 1] Check if isDead
  (if (<= (Variables|Default|GetHealthPoints) 0.0)
    (Variables|Default|SetbIsDead true)
    (else
      (Variables|Default|SetbIsDead false))))

(fn ConstructionScript)

(fn UpdateHealthPoints
  (params (Delta :type Float%20%28single-precision%29))
  ;[1 1 1] Update health charcater
  (bind _output_get (Variables|Default|SetHealthPoints (+ Delta (Variables|Default|GetHealthPoints))))
  (if (<= _output_get 0.0)
    (Variables|Default|SetbIsDead true)
    (else
      (Variables|Default|SetbIsDead false)))
  (return _output_get))