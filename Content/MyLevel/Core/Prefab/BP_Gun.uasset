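; BP_Gun is an automatic gun that fires BP_Projectile actors at a set fire rate while firing is active.
; StartFiring passes a DoOnce gate, fires immediately, then repeats FireProjectile on a looping timer set by FireRate.
; Each shot spawns a projectile at ProjectileSpawnPoint and plays an attached fire cue with its Type parameter set.
; StopFiring clears the timer and resets the gate.
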(event Custom|FireProjectile
  ;[1 1 1] Instantiate Projectile
  (Game|SpawnActorfromClass "/Game/MyLevel/Core/Prefab/BP_Projectile.BP_Projectile_C" (Transformation|GetWorldTransform (Variables|Default|GetProjectileSpawnPoint)) "Undefined" 0 0)
  (bind _returnvalue (Audio|SpawnSoundAttached "/Game/MyLevel/Audio/A_FireProjectile_Cue.A_FireProjectile_Cue" (Variables|Default|GetProjectileSpawnPoint) "None" "0, 0, 0" "0, 0, 0" "SnapToTarget" true 1.0 1.0 0.0 0 0))
  (Effects|Components|ParticleSystem|SetIntParameter _returnvalue "Type" 1))

(event Custom|StartFiring
  ;[1 1 1] Shoot Projectile
  (Utilities|FlowControl|DoOnce false
    (:Completed
      (CallFunction|FireProjectile)
      (Utilities|Time|SetTimerbyFunctionName 0 "FireProjectile" (/ 1.0 (Variables|Default|GetFireRate)) true))))

(event Custom|StopFiring
  (Utilities|Time|ClearTimerbyFunctionName 0 "FireProjectile")
  ;[1 1 1] Shoot Projectile
  (Utilities|FlowControl|DoOnce false) ; enters at Reset
)

(fn ConstructionScript)