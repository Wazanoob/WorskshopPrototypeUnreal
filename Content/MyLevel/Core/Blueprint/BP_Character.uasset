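; BP_Character is a character Blueprint that tracks health and death state and applies a customizable body color.
; UpdateHealthPoints adds a delta to health, sets IsDead at zero or below and returns the new health, while GetIsDead exposes the flag.
; The Construction Script creates dynamic materials for body and logo slots, tinting both with BodyColor.
; TriggerDeath is an empty event, and UpdateIsDead repeats the death check.
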(event Custom|UpdateIsDead
  ;[1 1 1] Check if isDead
  (if (<= (Variables|Default|GetHealthPoints) 0.0)
    (Variables|Default|SetbIsDead true)
    (else
      (Variables|Default|SetbIsDead false))))

(event Custom|TriggerDeath)

(event EventBeginPlay)

(event Collision|EventActorBeginOverlap
  (params (OtherActor :type Actor%20Object%20Reference)))

(event EventTick
  (params (DeltaSeconds :type Float%20%28single-precision%29)))

(fn ConstructionScript
  (CallFunction|InitializeBodyColor))

(fn UpdateHealthPoints
  (params (Delta :type Float%20%28single-precision%29))
  ;[1 1 1] Update health charcater
  (bind _output_get (Variables|Default|SetHealthPoints (+ Delta (Variables|Default|GetHealthPoints))))
  (if (<= _output_get 0.0)
    (Variables|Default|SetbIsDead true)
    (else
      (Variables|Default|SetbIsDead false)))
  (return _output_get))

(fn InitializeBodyColor
  ;[1 1 1] Change Body Color
  (bind _returnvalue (Rendering|Material|CreateDynamicMaterialInstance (Variables|Character|GetMesh) 0 0 "None" :!class /Script/Engine.PrimitiveComponent))
  (bind _output_get (Variables|Default|SetBodyMaterial _returnvalue))
  (Rendering|Material|SetVectorParameterValue _output_get "BodyColor" (Variables|Default|GetBodyColor) :!class /Script/Engine.MaterialInstanceDynamic)
  ;[1 1 1] Change Logo Color
  (bind _returnvalue_2 (Rendering|Material|CreateDynamicMaterialInstance (Variables|Character|GetMesh) 1 0 "None" :!class /Script/Engine.PrimitiveComponent))
  (bind _output_get_2 (Variables|Default|SetLogoMaterial _returnvalue_2))
  (Rendering|Material|SetVectorParameterValue _output_get_2 "BodyColor" (Variables|Default|GetBodyColor) :!class /Script/Engine.MaterialInstanceDynamic)
  (return))

(fn GetIsDead
  (return (Variables|Default|GetbIsDead)))